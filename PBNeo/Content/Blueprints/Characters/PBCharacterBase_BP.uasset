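; Base character Blueprint that adds camera post-process effects and relays combat events to first- and third-person animation Blueprints.
; On BeginPlay it creates dynamic outline, scope and custom-depth materials as zero-weight camera blendables.
; Releasing K toggles all three on or off together through a FlipFlop.
; Hit notifications reach the third-person AnimBP, while weapon-equip notifications pass the weapon to both AnimBPs.
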(event `self.ReceiveBeginPlay`
  (`|ExecutionSequence`
    (:`then_0`
      (bind _returnvalue (`KismetMaterialLibrary.CreateDynamicMaterialInstance` "/Game/Environment/Postprocess/PPM_Outline_A_Mat_Inst.PPM_Outline_A_Mat_Inst"))
      (bind _output_get (set `self.M_Outline` _returnvalue))
      (`CameraComponent.AddOrUpdateBlendable` (`self.CameraComp`) _output_get 0.0))
    (:`then_1`
      (bind _returnvalue_2 (`KismetMaterialLibrary.CreateDynamicMaterialInstance` "/Game/Environment/Postprocess/PPM_Scope_A_Mat_Inst.PPM_Scope_A_Mat_Inst"))
      (bind _output_get_2 (set `self.M_ScopeView` _returnvalue_2))
      (`CameraComponent.AddOrUpdateBlendable` (`self.CameraComp`) _output_get_2 0.0))
    (:`then_2`
      (bind _returnvalue_3 (`KismetMaterialLibrary.CreateDynamicMaterialInstance` "/Game/Environment/Postprocess/PPM_CustomDepthView_Mat_Inst.PPM_CustomDepthView_Mat_Inst"))
      (bind _output_get_3 (set `self.M_DepthView` _returnvalue_3))
      (`CameraComponent.AddOrUpdateBlendable` (`self.CameraComp`) _output_get_3 0.0))))

(event `Key|K`
  (params (Key :type "Key Structure" :default "AnyKey"))
  (:`Released`
    (`/Engine/EditorBlueprintResources/StandardMacros.FlipFlop`
      (:`A`
        (`CameraComponent.AddOrUpdateBlendable` (`self.CameraComp`) (`self.M_Outline`) 1.0)
        (`CameraComponent.AddOrUpdateBlendable` (`self.CameraComp`) (`self.M_DepthView`) 1.0)
        (`CameraComponent.AddOrUpdateBlendable` (`self.CameraComp`) (`self.M_ScopeView`) 1.0))
      (:`B`
        (`CameraComponent.AddOrUpdateBlendable` (`self.CameraComp`) (`self.M_Outline`) 0.0)
        (`CameraComponent.AddOrUpdateBlendable` (`self.CameraComp`) (`self.M_DepthView`) 0.0)
        (`CameraComponent.AddOrUpdateBlendable` (`self.CameraComp`) (`self.M_ScopeView`) 0.0)))))

(event `self.ReceiveTick`
  (params (DeltaSeconds :type "Float (single-precision)")))

(event `self.PlayHitEffects`
  (bind _mesh (`self.Mesh`))
  (bind _returnvalue (`SkeletalMeshComponent.GetAnimInstance` _mesh))
  ;[1 1 1] Notify Event
  (`/Engine/EditorBlueprintResources/StandardMacros.IsValid` _mesh
    (:`Is Valid`
      (`/Engine/EditorBlueprintResources/StandardMacros.IsValid` _returnvalue
        (:`Is Valid`
          (bind _aspbcharacter_base_3pv_anim_bp (cast `/Game/PBCharacterAnimations/PBCharacterBase_3PV_AnimBP` _returnvalue))
          (`/Game/PBCharacterAnimations/PBCharacterBase_3PV_AnimBP.OnHit` _aspbcharacter_base_3pv_anim_bp))))))

(event `self.NotifyEquipWeapon`
  (params (EquippedWeapon :type "PBWeapon Object Reference"))
  (bind _mesh (`self.Mesh`))
  (bind _mesh1p (`self.Mesh1P`))
  (bind _returnvalue (`SkeletalMeshComponent.GetAnimInstance` _mesh))
  (bind _returnvalue_2 (`SkeletalMeshComponent.GetAnimInstance` _mesh1p))
  ;[1 1 1] Notify Event
  (`|ExecutionSequence`
    (:`then_0`
      (`/Engine/EditorBlueprintResources/StandardMacros.IsValid` _mesh1p
        (:`Is Valid`
          (`/Engine/EditorBlueprintResources/StandardMacros.IsValid` _returnvalue_2
            (:`Is Valid`
              (bind _aspbcharacter_base_1pv_anim_bp (cast `/Game/PBCharacterAnimations/PBCharacterBase_1PV_AnimBP` _returnvalue_2))
              (`/Game/PBCharacterAnimations/PBCharacterBase_1PV_AnimBP.OnEquipWeapon` _aspbcharacter_base_1pv_anim_bp EquippedWeapon))))))
    (:`then_1`
      (`/Engine/EditorBlueprintResources/StandardMacros.IsValid` _mesh
        (:`Is Valid`
          (`/Engine/EditorBlueprintResources/StandardMacros.IsValid` _returnvalue
            (:`Is Valid`
              (bind _aspbcharacter_base_3pv_anim_bp (cast `/Game/PBCharacterAnimations/PBCharacterBase_3PV_AnimBP` _returnvalue))
              (`/Game/PBCharacterAnimations/PBCharacterBase_3PV_AnimBP.OnEquipWeapon` _aspbcharacter_base_3pv_anim_bp EquippedWeapon))))))))

(fn `UserConstructionScript`)