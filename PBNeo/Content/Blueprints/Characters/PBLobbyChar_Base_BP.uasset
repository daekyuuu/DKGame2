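; Base lobby character Blueprint that keeps its animation in step with mesh and weapon changes.
; On a mesh change notification it optionally plays a montage.
; On weapon equip, a helper passes the weapon to the first-person and third-person Anim Blueprints, after validating each mesh and anim instance and casting to the expected class.
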(event `self.NotifyMeshHasChanged`
  (params (bPlayAnimation :type Boolean))
  (if bPlayAnimation
    (`self.PlayAnimMontage` (`self.AnimMeshHasChanged`))))

(event `self.NotifyEquipWeapon`
  (params (EquippedWeapon :type "PBWeapon Object Reference"))
  (bind _mesh (`self.Mesh`))
  (bind _mesh1p (`self.Mesh1P`))
  (bind _returnvalue (`SkeletalMeshComponent.GetAnimInstance` _mesh))
  (bind _returnvalue_2 (`SkeletalMeshComponent.GetAnimInstance` _mesh1p))
  (`|ExecutionSequence`
    (:`then_0`
      (`/Engine/EditorBlueprintResources/StandardMacros.IsValid` _mesh1p
        (:`Is Valid`
          (`/Engine/EditorBlueprintResources/StandardMacros.IsValid` _returnvalue_2
            (:`Is Valid`
              (bind _aspbcharacter_base_1pv_anim_bp (cast `/Game/PBCharacterAnimations/PBCharacterBase_1PV_AnimBP` _returnvalue_2))
              (`/Game/PBCharacterAnimations/PBCharacterBase_1PV_AnimBP.OnEquipWeapon` _aspbcharacter_base_1pv_anim_bp EquippedWeapon))))))
    (:`then_1`
      (`/Engine/EditorBlueprintResources/StandardMacros.IsValid` _mesh
        (:`Is Valid`
          (`/Engine/EditorBlueprintResources/StandardMacros.IsValid` _returnvalue
            (:`Is Valid`
              (bind _aspbcharacter_base_3pv_anim_bp (cast `/Game/PBCharacterAnimations/PBCharacterBase_3PV_AnimBP` _returnvalue))
              (`/Game/PBCharacterAnimations/PBCharacterBase_3PV_AnimBP.OnEquipWeapon` _aspbcharacter_base_3pv_anim_bp EquippedWeapon))))))))

(fn `UserConstructionScript`)